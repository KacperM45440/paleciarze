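; Carryable box interactable that a character picks up and later releases back at a recorded spot.
; StartInteraction plays a carry montage, registers the box as the player's LastBoxPicked, attaches it to LeftHandSocket and eases it into place.
; EndInteraction stops a montage and calls DropBox, where a downward trace ahead only gates detaching.
; The box teleports to LastBoxPicked's BeginPlay location with a fixed Z offset; the move-to-hit node is unconnected.
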(event Custom|DropBox
  (bind _character (Variables|Default|GetCharacter))
  (bind _returnvalue (Transformation|GetActorLocation _character))
  (bind _returnvalue_2 (Transformation|GetActorForwardVector _character))
  (bind _returnvalue_3 (* _returnvalue_2 1e+02))
  (bind _returnvalue_4 (+ _returnvalue _returnvalue_3))
  (bind (_outhit _returnvalue_5) (Collision|LineTraceByChannel _returnvalue_4 (+ _returnvalue_4 "0.000000,0.000000,-500.000000") "TraceTypeQuery1" false 0 "None"))
  (if _returnvalue_5
    (Transformation|DetachFromActor "KeepWorld" "KeepWorld" "KeepWorld")
    (bind _returnvalue_6 (Actor|GetActorOfClass "/Game/ThirdPerson/Blueprints/BP_ThirdPersonCharacter.BP_ThirdPersonCharacter_C"))
    (bind _asbp_interactable_box (Utilities|Casting|CastToBP_Interactable_Box (Variables|/Game/ThirdPerson/Blueprints/BP_ThirdPersonCharacter.BP_ThirdPersonCharacter_C|GetLastBoxPicked _returnvalue_6)))
    (Transformation|Teleport (- (Variables|BP_Interactable_Box_C|GetBoxLocationVar _asbp_interactable_box) "0.000000,0.000000,182.000000") "0, 0, 0")))

(event EventBeginPlay
  (Variables|Default|SetBoxLocationVar (Transformation|GetWorldLocation (Variables|Default|GetBox))))

(event EventStartInteraction
  (params (ChracterInteract :type Actor%20Object%20Reference))
  (|CallParentFunction ChracterInteract)
  (bind _ascharacter (Utilities|Casting|CastToCharacter (Variables|Default|GetInteractingActor)))
  (Variables|Default|SetCharacter _ascharacter)
  (Animation|Montage|PlayMontage (Variables|/Script/Engine.Character|GetMesh _ascharacter) "/Game/Characters/Worker_KM/Pal_RetCarring_Montage.Pal_RetCarring_Montage"
    (:then
      (bind _returnvalue (Actor|GetActorOfClass "/Game/ThirdPerson/Blueprints/BP_ThirdPersonCharacter.BP_ThirdPersonCharacter_C"))
      (Variables|/Game/ThirdPerson/Blueprints/BP_ThirdPersonCharacter.BP_ThirdPersonCharacter_C|SetLastBoxPicked _returnvalue self)
      (Transformation|AttachComponentToComponent (Variables|/Script/Engine.Character|GetMesh _ascharacter) "LeftHandSocket" "KeepWorld" "KeepWorld" "KeepWorld" true)
      (Components|MoveComponentTo (Variables|Default|GetDefaultSceneRoot) "0, 0, 0" "0, 0, 0" true true 0.3 true))))

(fn ConstructionScript
  (|CallParentFunction))

(fn EndInteraction
  (|CallParentFunction)
  (bind _character (Variables|Default|GetCharacter)
    (:then
      (Animation|StopAnimMontage _character "/Game/Characters/Mannequins/Animations/Quinn/Carring_Montage.Carring_Montage")
      (CallFunction|DropBox)
      (return true))
    (:else)))