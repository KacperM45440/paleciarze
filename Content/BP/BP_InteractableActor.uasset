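; Interactable actor that lets the player start and end an interaction with the E key while tracking whether it is occupied.
; When unoccupied, a box overlap by a player, checked through an IsPlayer message, shows a cached instruction widget and enables actor input; leaving reverses both.
; Starting an interaction stores the character, marks the actor occupied and hides the prompt.
; MarkasOccupied and IsAvailable expose occupancy for external claiming and queries.
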(event OnComponentBeginOverlap(Box)
  (params (OverlappedComponent :type Primitive%20Component%20Object%20Reference) (OtherActor :type Actor%20Object%20Reference) (OtherComp :type Primitive%20Component%20Object%20Reference) (OtherBodyIndex :type Integer) (bFromSweep :type Boolean) (SweepResult :type Hit%20Result%20Structure%20%28by%20ref%29))
  (if (not (Variables|Default|GetOccupied))
    (bind _yes_no (Class|BPLCharacter|IsPlayer?(Message) OtherActor))
    (if _yes_no
      (Variables|Default|SetInteractingActor OtherActor)
      (Variables|Default|GetInstruction_Widget
        (:then
          _)
        (:else
          (bind _returnvalue (UserInterface|CreateWidget "/Game/BP/Instruction.Instruction_C"))
          (Variables|Default|SetInstruction_Widget _returnvalue)))
      (UserInterface|Viewport|AddtoViewport (Variables|Default|GetInstruction_Widget) 0)
      (Input|EnableInput (Game|GetPlayerController 0)))))

(event OnComponentEndOverlap(Box)
  (params (OverlappedComponent :type Primitive%20Component%20Object%20Reference) (OtherActor :type Actor%20Object%20Reference) (OtherComp :type Primitive%20Component%20Object%20Reference) (OtherBodyIndex :type Integer))
  (bind _yes_no (Class|BPLCharacter|IsPlayer?(Message) OtherActor))
  (if _yes_no
    (Utilities|HideInstruction
      (:then
        (Input|DisableInput (Game|GetPlayerController 0))))))

(event EventBeginPlay)

(event Collision|EventActorBeginOverlap
  (params (OtherActor :type Actor%20Object%20Reference)))

(event EventTick
  (params (DeltaSeconds :type Float%20%28single-precision%29)))

(event EventStartInteraction
  (params (ChracterInteract :type Actor%20Object%20Reference))
  (Variables|Default|SetOccupied true)
  (Variables|Default|SetInteractingActor ChracterInteract)
  (Variables|Default|SetInteracting true)
  (Utilities|HideInstruction))

(event EventMarkasOccupied
  (Variables|Default|SetOccupied true))

(event Input|KeyboardEvents|E
  (params (Key :type Key%20Structure :default "None"))
  (:Pressed
    (if (Variables|Default|GetInteracting)
      (CallFunction|EndInteraction)
      (else
        (CallFunction|StartInteraction (Variables|Default|GetInteractingActor))))))

(fn ConstructionScript)

(fn EndInteraction
  (Variables|Default|SetInteracting false)
  (Variables|Default|SetOccupied false)
  (return true))

(fn IsAvailable?
  (return (not (Variables|Default|GetOccupied))))