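; Manager Blueprint that periodically randomizes a field index and drives a highlight color through a material parameter collection.
; BeginPlay applies M_Highlight to Box and starts a looping timer on RandomizeField, which rolls an index and calls HighlightField.
; HighlightField rolls again, then switches on the index to set the Color parameter in MPC_Highlight, with debug prints.
; All indices in the rolled range share one color; only the default branch uses another.
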(event Custom|HighlightField
  (bind _output_get (Variables|Default|SetRandomFieldIndex (Math|Random|RandomIntegerinRange 0 7)))
  (switch int _output_get
    (:Default
      (Development|PrintString "default")
      (Rendering|Material|SetVectorParameterValue "/Game/Materials/MPC_Highlight.MPC_Highlight" "Color" (Math|Conversions|ToLinearColor(Color) (Variables|Default|GetNewVar)) :!class /Script/Engine.KismetMaterialLibrary)
      (Development|PrintString "set defult"))
    (:0
      (Rendering|Material|SetVectorParameterValue "/Game/Materials/MPC_Highlight.MPC_Highlight" "Color" (Math|Conversions|ToLinearColor(Color) (Variables|Default|GetNewVar_0)) :!class /Script/Engine.KismetMaterialLibrary :!label _label)
      (Development|PrintString "0-7"))
    (:1
      (goto _label))
    (:2
      (goto _label))
    (:3
      (goto _label))
    (:4
      (goto _label))
    (:5
      (goto _label))
    (:6
      (goto _label))
    (:7
      (goto _label))))

(event Custom|RandomizeField
  (Variables|Default|SetRandomFieldIndex (Math|Random|RandomIntegerinRange 0 7))
  (CallFunction|HighlightField))

(event EventBeginPlay
  (Utilities|Time|SetTimerbyFunctionName 0 "RandomizeField" 2.0 true)
  (Rendering|Material|SetMaterial (Variables|Default|GetBox) 0 "/Game/Materials/M_Highlight.M_Highlight"))

(fn ConstructionScript)