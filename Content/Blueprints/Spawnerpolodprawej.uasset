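; Spawner actor that repeatedly spawns BP_Forkliftprawo forklifts for as long as it runs.
; BeginPlay calls Resp2 immediately, then loops it on a timer whose 2–5 second interval is randomized only once.
; The first forklift spawns at the StaticMesh location; the Czybylrespawn flag makes later ones use a hardcoded world Y with the mesh's X and Z.
; The spawn loop runs a single iteration, and the Resp function is empty.
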(event Custom|Resp2
  (bind _staticmesh (Variables|Default|GetStaticMesh))
  (bind _returnvalue (Transformation|GetWorldLocation _staticmesh))
  (for _index (range 0 0)
    (Variables|Default|SetSpawnLocation (Math|Vector|MakeVector (+ (* _index 0) (.x _returnvalue)) (.y _returnvalue) (.z _returnvalue)))
    (if (Math|Integer|InRange(Integer) _index 0 3)
      (if (Variables|Default|Getczybylrespawn)
        (bind _output_get (Variables|Default|SetSpawnLocation (Math|Vector|MakeVector (.x (Variables|Default|GetSpawnLocation)) 1.13e+03 (.z (Variables|Default|GetSpawnLocation)))))
        (Game|SpawnActorfromClass "/Game/Blueprints/BP_Forkliftprawo.BP_Forkliftprawo_C" (Math|Transform|MakeTransform _output_get "0, 0, 0" "1.000000,1.000000,1.000000") "Undefined" "MultiplyWithRoot" 0 0)
        (else
          (bind _output_get_2 (Variables|Default|SetSpawnLocation (Variables|Default|GetSpawnLocation)))
          (Game|SpawnActorfromClass "/Game/Blueprints/BP_Forkliftprawo.BP_Forkliftprawo_C" (Math|Transform|MakeTransform _output_get_2 "0, 0, 0" "1.000000,1.000000,1.000000") "Undefined" "MultiplyWithRoot" 0 0)
          (Variables|Default|Setczybylrespawn true))))))

(event EventBeginPlay
  (CallFunction|Resp2)
  (Utilities|Time|SetTimerbyFunctionName 0 "Resp2" (Math|Random|RandomFloatinRange 2.0 5.0) true))

(fn ConstructionScript)

(fn Resp)