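; BP_FloorRow is a row of eight floor tiles with one randomly chosen hazard field that teleports the player character.
; A two-second looping timer picks an index, sets the highlight color in a Material Parameter Collection, and enables collision only on that field's box.
; Nested loops assign dynamic highlight or default materials to the Podloga tiles.
; An actor overlap by BP_TopDownCharacter teleports it to a fixed location.
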(event Custom|HighlightField
  (bind _output_get (Variables|Default|SetRandomFieldIndex (Math|Random|RandomIntegerinRange 0 7)))
  (Rendering|Material|SetVectorParameterValue "/Game/Materials/MPC_Highlight.MPC_Highlight" "Color" (Math|Conversions|ToLinearColor(Color) (Variables|Default|GetNewVar_0)) :!class /Script/Engine.KismetMaterialLibrary)
  (for (_array_element _array_index) (Utilities|Array|MakeArray (Variables|Default|GetBox1) (Variables|Default|GetBox2) (Variables|Default|GetBox3) (Variables|Default|GetBox4) (Variables|Default|GetBox5) (Variables|Default|GetBox6) (Variables|Default|GetBox7) (Variables|Default|GetBox8))
    (if (== _array_index _output_get)
      (Collision|SetCollisionEnabled _array_element (Variables|Default|GetNew%20Type))
      (bind _returnvalue (Rendering|Material|CreateDynamicMaterialInstance "/Game/Materials/MI_Highlight.MI_Highlight" "None" "None" :!class /Script/Engine.KismetMaterialLibrary))
      (else
        (Collision|SetCollisionEnabled _array_element "NoCollision")
        (bind _returnvalue_2 (Rendering|Material|CreateDynamicMaterialInstance "/Game/Materials/MI_FloorMats01.MI_FloorMats01" "None" "None" :!class /Script/Engine.KismetMaterialLibrary))))
    (for (_array_element_2 _array_index_2) (Utilities|Array|MakeArray (Variables|Default|Getpodloga1) (Variables|Default|Getpodloga2) (Variables|Default|Getpodloga3) (Variables|Default|Getpodloga4) (Variables|Default|Getpodloga5) (Variables|Default|Getpodloga6) (Variables|Default|Getpodloga7) (Variables|Default|Getpodloga8))
      (if (== _array_index_2 _output_get)
        (Rendering|Material|SetMaterial _array_element_2 0 _returnvalue)
        (else
          (Rendering|Material|SetMaterial _array_element_2 0 _returnvalue_2))))))

(event Custom|RandomizeField
  (CallFunction|HighlightField))

(event EventBeginPlay
  (Utilities|Time|SetTimerbyFunctionName 0 "RandomizeField" 2.0 true))

(event Collision|EventActorBeginOverlap
  (params (OtherActor :type Actor%20Object%20Reference))
  (bind _asbp_top_down_character (Utilities|Casting|CastToBP_TopDownCharacter OtherActor))
  (Transformation|Teleport _asbp_top_down_character (Math|Vector|MakeVector 2e+03 1e+03 0.0) "0, 0, 0"))

(fn ConstructionScript)