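; SoundController selects which music track plays when a level begins.
; On BeginPlay it compares the current level name to "MainMenu", then plays either the MenuMusic or Level1Music audio component and stops the other.
; Any level not named MainMenu gets the Level 1 music, and the choice is made only once, with no crossfade.
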(event EventBeginPlay
  (bind _level1music (Variables|Default|GetLevel1Music))
  (bind _menumusic (Variables|Default|GetMenuMusic))
  (bind _audiocomponent (Variables|/Script/Engine.AmbientSound|GetAudioComponent _level1music))
  (bind _audiocomponent_2 (Variables|/Script/Engine.AmbientSound|GetAudioComponent _menumusic))
  (bind _returnvalue (Game|GetCurrentLevelName true))
  (if (Utilities|Enum|Equal(Enum) _returnvalue "MainMenu")
    (Audio|Components|Audio|Play _audiocomponent_2 0.0)
    (Audio|Components|Audio|Stop _audiocomponent)
    (else
      (Audio|Components|Audio|Play _audiocomponent 0.0)
      (Audio|Components|Audio|Stop _audiocomponent_2))))

(fn ConstructionScript)