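; Hazard spawner ("polasmierciprawo") that repeatedly spawns a Forklift, then Kolce (spikes) at the same point two seconds later.
; Resp2 runs on BeginPlay and a looping timer, using the StaticMesh location for the first spawn.
; Later spawns keep the mesh's X and Z but take Y from Ymin, which a separate looping timer randomizes among four fixed positions.
; The spawn loop covers one index, and Resp is empty.
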(event Custom|Resp2
  (bind _staticmesh (Variables|Default|GetStaticMesh))
  (bind _returnvalue (Transformation|GetWorldLocation _staticmesh))
  (for _index (range 0 0)
    (Variables|Default|SetSpawnLocation (Math|Vector|MakeVector (+ (* _index 100) (.x _returnvalue)) (.y _returnvalue) (.z _returnvalue)))
    (if (Math|Integer|InRange(Integer) _index 0 3)
      (if (Variables|Default|Getczybylrespawn)
        (bind _output_get (Variables|Default|SetSpawnLocation (Math|Vector|MakeVector (.x (Variables|Default|GetSpawnLocation)) (Variables|Default|Getymin) (.z (Variables|Default|GetSpawnLocation)))))
        (Game|SpawnActorfromClass "/Game/Blueprints/Forklift.Forklift_C" (Math|Transform|MakeTransform _output_get "0, 0, 0" "1.000000,1.000000,1.000000") "Undefined" "MultiplyWithRoot" 0 0)
        (Utilities|FlowControl|Delay 2.0)
        (Game|SpawnActorfromClass "/Game/Blueprints/Kolce.Kolce_C" (Math|Transform|MakeTransform _output_get "0, 0, 0" "1.000000,1.000000,1.000000") "Undefined" "MultiplyWithRoot" 0 0)
        (else
          (bind _output_get_2 (Variables|Default|SetSpawnLocation (Variables|Default|GetSpawnLocation)))
          (Game|SpawnActorfromClass "/Game/Blueprints/Forklift.Forklift_C" (Math|Transform|MakeTransform _output_get_2 "0, 0, 0" "1.000000,1.000000,1.000000") "Undefined" "MultiplyWithRoot" 0 0)
          (Utilities|FlowControl|Delay 2.0)
          (Game|SpawnActorfromClass "/Game/Blueprints/Kolce.Kolce_C" (Math|Transform|MakeTransform _output_get_2 "0, 0, 0" "1.000000,1.000000,1.000000") "Undefined" "MultiplyWithRoot" 0 0)
          (Variables|Default|Setczybylrespawn true))))))

(event Custom|Randomnum
  (bind _output_get (Variables|Default|SetRandomNumber (Math|Random|RandomIntegerinRange 0 3)))
  (switch int _output_get
    (:0
      (Variables|Default|Setymin 1e+02))
    (:1
      (Variables|Default|Setymin 3e+02))
    (:2
      (Variables|Default|Setymin 5e+02))
    (:3
      (Variables|Default|Setymin 7e+02))))

(event EventBeginPlay
  (CallFunction|Resp2)
  (Utilities|Time|SetTimerbyFunctionName 0 "Resp2" 6.0 true)
  (Utilities|Time|SetTimerbyFunctionName 0 "Randomnum" 5.0 true))

(fn ConstructionScript)

(fn Resp)