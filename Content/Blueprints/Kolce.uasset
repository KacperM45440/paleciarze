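; Spike hazard (Kolce) that ragdolls the third-person character on overlap, then after a second restores it and teleports it to a hardcoded reset point.
; If the character's last picked box is valid, it also drops that box, stops the carry montage and clears HasBox.
; On BeginPlay two chained timelines move the spikes vertically, and a timer-triggered delayed event destroys the actor about six seconds later.
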(event Custom|DestroyActor
  (Utilities|FlowControl|Delay 5.0)
  (Actor|DestroyActor))

(event EventBeginPlay
  (Utilities|Time|SetTimerbyFunctionName 0 "DestroyActor" 1.0 true)
  (bind _goradol (Timeline|Timeline Play)
    (:Update
      (Transformation|AddActorWorldOffset (Math|Vector|MakeVector 0.0 0.0 _goradol))
      (Utilities|FlowControl|Delay 0.5)
      (bind _dol (Timeline|Timeline_0 Play)
        (:Update
          (Transformation|AddActorWorldOffset (Math|Vector|MakeVector 0.0 0.0 _dol)))))))

(event EventTick
  (params (DeltaSeconds :type Float%20%28single-precision%29)))

(event Collision|EventActorBeginOverlap
  (params (OtherActor :type Actor%20Object%20Reference))
  (bind _returnvalue (Math|Vector|MakeVector 3.2e+03 1e+02 1.5e+02))
  (bind _asbp_third_person_character (Utilities|Casting|CastToBP_ThirdPersonCharacter OtherActor))
  (bind _asbp_interactable_box (Utilities|Casting|CastToBP_Interactable_Box (Variables|/Game/ThirdPerson/Blueprints/BP_ThirdPersonCharacter.BP_ThirdPersonCharacter_C|GetLastBoxPicked _asbp_third_person_character))
    (:then
      (Default|EndInteraction _asbp_interactable_box)
      (Default|DropBox _asbp_interactable_box)
      (Default|Radgdoll _asbp_third_person_character)
      (Utilities|FlowControl|Delay 1.0)
      (bind _returnvalue_2 (Actor|GetActorOfClass "/Game/ThirdPerson/Blueprints/BP_ThirdPersonCharacter.BP_ThirdPersonCharacter_C"))
      (Default|UnRadgdoll _returnvalue_2)
      (Transformation|Teleport _returnvalue_2 _returnvalue "0, 0, 0")
      (bind _returnvalue_3 (Actor|GetActorOfClass "/Game/ThirdPerson/Blueprints/BP_ThirdPersonCharacter.BP_ThirdPersonCharacter_C"))
      (Animation|Montage|MontageStop (Components|SkeletalMesh|GetAnimInstance (Variables|/Script/Engine.Character|GetMesh _returnvalue_3)) 0.0 "/Game/Characters/Worker_KM/Pal_RetCarring_Montage.Pal_RetCarring_Montage")
      (bind _returnvalue_4 (Actor|GetActorOfClass "/Game/ThirdPerson/Blueprints/BP_ThirdPersonCharacter.BP_ThirdPersonCharacter_C"))
      (Variables|/Game/ThirdPerson/Blueprints/BP_ThirdPersonCharacter.BP_ThirdPersonCharacter_C|SetHasBox _returnvalue_4 false))
    (:CastFailed
      (Default|Radgdoll _asbp_third_person_character)
      (Utilities|FlowControl|Delay 1.0)
      (bind _returnvalue_5 (Actor|GetActorOfClass "/Game/ThirdPerson/Blueprints/BP_ThirdPersonCharacter.BP_ThirdPersonCharacter_C"))
      (Default|UnRadgdoll _returnvalue_5)
      (Transformation|Teleport _returnvalue_5 _returnvalue "0, 0, 0"))))

(fn ConstructionScript)